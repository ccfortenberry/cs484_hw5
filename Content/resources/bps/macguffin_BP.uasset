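; Macguffin collectible actor that rotates in the world until the player character picks it up.
; Each tick adds a world pitch rotation equal to delta time plus its current pitch, so the spin is not a constant rate.
; A hit from Character_Blueprint destroys the actor, then flags MacguffinCollected on gamemode_BP.
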(event EventBeginPlay)

(event Collision|EventActorBeginOverlap
  (params (OtherActor :type Actor%20Object%20Reference)))

(event EventTick
  (params (DeltaSeconds :type Float%20%28single-precision%29))
  (Class|Actor|AddActorWorldRotation (Math|Rotator|MakeRotator 0.0 (+ DeltaSeconds (.Pitch (Math|Rotator|BreakRotator (Transformation|GetActorRotation)))) 0.0)))

(event Collision|EventHit
  (params (MyComp :type Primitive%20Component%20Object%20Reference) (Other :type Actor%20Object%20Reference) (OtherComp :type Primitive%20Component%20Object%20Reference) (bSelfMoved :type Boolean) (HitLocation :type Vector :default "0, 0, 0") (HitNormal :type Vector :default "0, 0, 0") (NormalImpulse :type Vector :default "0, 0, 0") (Hit :type Hit%20Result%20Structure%20%28by%20ref%29))
  (Utilities|Casting|CastToCharacter_Blueprint Other)
  (Actor|DestroyActor)
  (bind _asgamemode_bp (Utilities|Casting|CastTogamemode_BP (Game|GetGameMode)))
  (Variables|/Game/resources/bps/gamemode_BP.gamemode_BP_C|SetmacguffinCollected _asgamemode_bp true))

(fn ConstructionScript)