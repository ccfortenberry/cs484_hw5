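; Game mode Blueprint that respawns the player character after it is destroyed.
; On BeginPlay it binds to the destroyed event of the current player's Character_Blueprint.
; When that fires, it waits briefly, spawns a new character at a SpawnTransform, has the player controller possess it, and rebinds the event for the next death.
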(event Custom|OnDestoyed_Event_0
  (params (DestroyedActor :type Actor%20Object%20Reference))
  (Utilities|FlowControl|Delay 2.0)
  (bind _returnvalue (Game|SpawnActorfromClass "/Game/resources/bps/Character_Blueprint.Character_Blueprint_C" (Variables|Default|GetspawnTransform) "Undefined" 0 0))
  (Pawn|Possess (Game|GetPlayerController 0) _returnvalue)
  (CallFunction|Respawn))

(event Custom|Respawn
  (bind _ascharacter_blueprint (Utilities|Casting|CastToCharacter_Blueprint (Game|GetPlayerCharacter 0)))
  (Game|BindEventtoOnDestroyed _ascharacter_blueprint (delegate Custom|OnDestoyed_Event_0)))

(event EventBeginPlay
  (bind _ascharacter_blueprint (Utilities|Casting|CastToCharacter_Blueprint (Game|GetPlayerCharacter 0)))
  (Game|BindEventtoOnDestroyed _ascharacter_blueprint (delegate Custom|OnDestoyed_Event_0)))

(event EventTick
  (params (DeltaSeconds :type Float%20%28single-precision%29)))

(fn ConstructionScript)